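; Aim-assist actor for the Hillbilly killer that snaps the player's view onto the nearest CamperPlayer on a chainsaw swing.
; The swing triggers assist only when that camper is within range and inside pitch and yaw tolerances of the control rotation.
; Tick then lerps control rotation toward the camper's live, height-offset position with square-root easing, switching itself off near completion.
; BeginPlay still spawns an unused debug marker.
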(event `Initialize`
  (params (InOwningKiller :type "SlasherPlayer Object Reference"))
  (bind _output_get (set `self.OwningKiller` InOwningKiller))
  (set `self.PlayerController` (`DBDPlayer.GetPlayerController` _output_get)))

(event `OnChainsawSwing`
  (bind (_distance _camperplayer) (`self.GetNearestCamper`))
  (bind _deltaangles (`self.GetDeltaViewAngles` (`self.GetViewAnglesBetweenTwoObjects` (`self.GetActorEyesViewPoint` (`self.OwningKiller`)) (`self.GetCamperLocation` _camperplayer))))
  (set `self.HitCamper` _camperplayer)
  (if (`self.IsChainsawHit` _distance _deltaangles)
    (`self.InterpRotation` _deltaangles)))

(event `InterpRotation`
  (params (Target :type "Rotator Structure"))
  (set `self.TargetRotation` Target)
  (set `self.CurrentRotation` (`Controller.GetControlRotation` (`self.PlayerController`)))
  (set `self.InterpAlpha` 0.0)
  (`self.SetActorTickEnabled` true))

(event `self.ReceiveTick`
  (params (DeltaSeconds :type "Float (single-precision)"))
  ;[1 1 1] Handles Control Rotation interpolation
  (bind _output_get (set `self.InterpAlpha` (+ (`self.InterpAlpha`) (* DeltaSeconds (`self.InterpSpeed`)))))
  (`Controller.SetControlRotation` (`self.PlayerController`) (`KismetMathLibrary.RLerp` (`self.CurrentRotation`) (`self.GetViewAnglesBetweenTwoObjects` (`self.GetActorEyesViewPoint` (`self.OwningKiller`)) (`self.GetCamperLocation` (`self.HitCamper`))) (`KismetMathLibrary.Sqrt` _output_get) true))
  (if (>= (`self.InterpAlpha`) 0.99)
    (`self.SetActorTickEnabled` false)
    (set `self.HitCamper` null)))

(event `self.ReceiveBeginPlay`
  ;[1 1 1] Visualizing aim point (not used)
  (bind _returnvalue (`|SpawnActorFromClass` "/Game/HillbillyAimAssist/BP_Point.BP_Point_C" (`KismetMathLibrary.MakeTransform` (0.0 0.0 0.0)) "Undefined" "OverrideRootScale" null null))
  (set `self.CamperMarker` _returnvalue))

(fn `GetAimTargetLocation`
  (params (Camper :type "CamperPlayer Object Reference"))
  (returns (ReturnValue :type "Vector Structure"))
  (return (+ (+ (`self.K2_GetActorLocation` Camper) (0.0 0.0 25.0)) (* (`self.GetActorForwardVector` Camper) 25.0))))

(fn `GetCamperLocation`
  (params (Camper :type "CamperPlayer Object Reference"))
  (returns (ReturnValue :type "Vector Structure"))
  (return (+ (`self.K2_GetActorLocation` Camper) (0.0 0.0 35.0))))

(fn `GetDeltaViewAngles`
  (params (InAngles :type "Rotator Structure"))
  (returns (DeltaAngles :type "Rotator Structure"))
  (return (`KismetMathLibrary.NormalizedDeltaRotator` InAngles (`Controller.GetControlRotation` (`self.PlayerController`)))))

(fn `GetNearestCamper`
  (returns (Distance :type "Float (double-precision)") (CamperPlayer :type "CamperPlayer Object Reference"))
  (bind _outactors (`GameplayStatics.GetAllActorsOfClass` "/Script/DeadByDaylight.CamperPlayer"))
  (bind (_distance _returnvalue) (`GameplayStatics.FindNearestActor` (`self.K2_GetActorLocation` (`self.OwningKiller`)) _outactors))
  (return _distance (cast `CamperPlayer` _returnvalue :!pure true)))

(fn `GetViewAnglesBetweenTwoObjects`
  (params (Start :type "Vector Structure") (Target :type "Vector Structure"))
  (returns (ViewAngles :type "Rotator Structure"))
  (bind (_returnvalue_x _returnvalue_y _returnvalue_z) (`KismetMathLibrary.BreakVector` (- Start Target)))
  (return (`KismetMathLibrary.MakeRotator` 0.0 (`KismetMathLibrary.DegAtan2` (- 0.0 _returnvalue_z) (`KismetMathLibrary.Hypotenuse` _returnvalue_x _returnvalue_y)) (+ (`KismetMathLibrary.DegAtan2` _returnvalue_y _returnvalue_x) 180.0))))

(fn `IsChainsawHit`
  (params (Distance :type "Float (double-precision)") (DeltaViewAngles :type "Rotator Structure"))
  (returns (Result :type Boolean))
  (bind (_deltaviewangles_roll _deltaviewangles_pitch _deltaviewangles_yaw) (`KismetMathLibrary.BreakRotator` (`local.DeltaViewAngles`)))
  (bind (_minimaldeltaanglestotrigger_roll _minimaldeltaanglestotrigger_pitch _minimaldeltaanglestotrigger_yaw) (`KismetMathLibrary.BreakRotator` (`self.MinimalDeltaAnglesToTrigger`)))
  (if (<= Distance (`self.NearestDistanceToTrigger`))
    (return (and (<= (`KismetMathLibrary.Abs` _deltaviewangles_pitch) _minimaldeltaanglestotrigger_pitch) (<= (`KismetMathLibrary.Abs` _deltaviewangles_yaw) _minimaldeltaanglestotrigger_yaw)))
    (else
      (return false))))

(fn `PrintDebugInfo`
  (params (Dist :type "Float (double-precision)") (InRot :type "Rotator Structure"))
  (`/Game/BetterHilbilly_LoggingUtilities/BlueprintLoggingLibrary.PrintString` (`KismetTextLibrary.Conv_TextToString` (`|FormatText` "Nearest Camper: {Dist}" Dist)))
  (`/Game/BetterHilbilly_LoggingUtilities/BlueprintLoggingLibrary.PrintString` (`KismetStringLibrary.Conv_RotatorToString` InRot) "NewEnumerator1"))

(fn `UserConstructionScript`)