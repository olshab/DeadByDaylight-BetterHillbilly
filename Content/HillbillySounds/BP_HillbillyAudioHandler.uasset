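; Hillbilly killer audio handler that plays chainsaw charge, rev, cancel, stop and hit sounds.
; A local killer gets layered audio components with timers and fades, while others mostly post Wwise events to the slasher audio component.
; Local revs chain through OnAudioFinished, picking single or multi by weighted random with a repeat cap.
; Tick calls chainsaw stop while the game is ended, as the GameEnd listener registration is unconnected.
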(event `self.ReceiveBeginPlay`
  (bind _output_get (set `self.IsLocalPlayer` (== (`self.OwningKiller`) (`GameplayStatics.GetPlayerCharacter` 0))))
  (if _output_get
    ;[1 1 1] sfx_chainsaw_attack_rev_single
    (bind _returnvalue (`AddComponent|NODE_AddAudioComponent-0` :`self` (`self.OwningKiller`)))
    (set `self.sfx_chainsaw_attack_rev_single` _returnvalue)
    ;[1 1 1] sfx_chainsaw_attack_rev_multi
    (bind _returnvalue_2 (`AddComponent|NODE_AddAudioComponent-1` :`self` (`self.OwningKiller`)))
    (set `self.sfx_chainsaw_attack_rev_multi` _returnvalue_2)
    ;[1 1 1] sfx_chainsaw_idle_loop
    (bind _returnvalue_3 (`AddComponent|NODE_AddAudioComponent-2` :`self` (`self.OwningKiller`)))
    (set `self.sfx_chainsaw_idle_loop` _returnvalue_3)
    ;[1 1 1] sfx_chainsaw_attack_body_loop_02
    (bind _returnvalue_4 (`AddComponent|NODE_AddAudioComponent-3` :`self` (`self.OwningKiller`)))
    (set `self.sfx_chainsaw_attack_body_loop` _returnvalue_4)
    ;[1 1 1] sfx_chainsaw_attack_start_add_01
    (bind _returnvalue_5 (`AddComponent|NODE_AddAudioComponent-4` :`self` (`self.OwningKiller`)))
    (set `self.sfx_chainsaw_attack_start_add` _returnvalue_5)
    ;[1 1 1] sfx_chainsaw_attack_start
    (bind _returnvalue_6 (`AddComponent|NODE_AddAudioComponent-5` :`self` (`self.OwningKiller`)))
    (set `self.sfx_chainsaw_attack_start` _returnvalue_6)))

(event `GameEnded`
  (params (gameEventType :type "GameplayTag Structure") (gameEventData :type "GameEventData Structure (by ref)")))

(event `AudioEvent_Chainsaw_Cancel`
  (set `self.IsChainsawCancelled` true)
  (if (`self.IsLocalPlayer`)
    (clear `AudioComponent.OnAudioFinished` (`self.sfx_chainsaw_attack_rev_single`))
    (clear `AudioComponent.OnAudioFinished` (`self.sfx_chainsaw_attack_rev_multi`))
    (`KismetSystemLibrary.K2_ClearAndInvalidateTimerHandle` (`self.rev_start_timer`))
    (`KismetSystemLibrary.K2_ClearAndInvalidateTimerHandle` (`self.first_rev_timer`))
    (`AudioComponent.FadeOut` (`self.sfx_chainsaw_attack_rev_single`) 0.5 0.0 "Linear")
    (`AudioComponent.FadeOut` (`self.sfx_chainsaw_attack_rev_multi`) 0.5 0.0 "Linear")
    (`AudioComponent.FadeOut` (`self.sfx_chainsaw_idle_loop`) 0.5 0.0 "Linear")
    (`AudioComponent.FadeOut` (`self.sfx_chainsaw_attack_start_add`) 0.5 0.0 "Linear")
    (`AudioComponent.FadeOut` (`self.sfx_chainsaw_attack_start`) 0.5 0.0 "Linear")
    (set `self.IsRevSinglePlaying` false)
    (set `self.IsRevMultiPlaying` false)
    (set `self.RevSingleContinuouslyPlayedNum` 0)
    (set `self.RevMultiContinuouslyPlayedNum` 0)
    (set `self.FirstRevPlayed` false)
    (`GameplayStatics.PlaySoundAtLocation` "/Game/HillbillySounds/SoundCues/sfx_chainsaw_stop.sfx_chainsaw_stop" (`self.K2_GetActorLocation` (`self.OwningKiller`)) (struct) 1.0 1.0 0.0 null null null)
    (else
      (bind _audio_component (message `/Game/Characters/Slashers/Blueprints/Interfaces/ISlasherEffectInterface.GetSlasherAudioComponent` (`self.OwningKiller`)))
      (`AkGameObject.PostAkEvent` _audio_component null 0 (delegate `CustomEvent2`) (`|MakeArray` (struct) :!type "AkExternalSourceInfo Structure") "")
      (`GameplayStatics.PlaySoundAtLocation` "/Game/HillbillySounds/SoundCues/sfx_chainsaw_stop_attenuation.sfx_chainsaw_stop_attenuation" (`self.K2_GetActorLocation` (`self.OwningKiller`)) (struct) 1.0 1.0 0.0 null null null))))

(event `CustomEvent2`
  (params (CallbackType :type "EAkCallbackType Enum" :default "EndOfEvent") (CallbackInfo :type "AkCallbackInfo Object Reference")))

(event `AudioEvent_Chainsaw_Charge`
  (set `self.IsChainsawCancelled` false)
  (if (`self.IsLocalPlayer`)
    (`AudioComponent.FadeIn` (`self.sfx_chainsaw_attack_start_add`) 0.3 0.7 0.0 "Linear")
    (bind _returnvalue (`KismetSystemLibrary.K2_SetTimerDelegate` (delegate `rev_start`) 0.05))
    (set `self.rev_start_timer` _returnvalue)
    (`AudioComponent.FadeIn` (`self.sfx_chainsaw_idle_loop`) 0.3 1.0 0.0 "Linear")
    (bind _returnvalue_2 (`KismetSystemLibrary.K2_SetTimerDelegate` (delegate `AudioEvent_Chainsaw_Rev`) 0.25))
    (set `self.first_rev_timer` _returnvalue_2)
    (add `AudioComponent.OnAudioFinished` (`self.sfx_chainsaw_attack_rev_single`) (delegate `AudioEvent_Chainsaw_Rev`))
    (add `AudioComponent.OnAudioFinished` (`self.sfx_chainsaw_attack_rev_multi`) (delegate `AudioEvent_Chainsaw_Rev`))
    (else
      (bind _audio_component (message `/Game/Characters/Slashers/Blueprints/Interfaces/ISlasherEffectInterface.GetSlasherAudioComponent` (`self.OwningKiller`)))
      (`AkGameObject.PostAkEvent` _audio_component null 0 (delegate `CustomEvent3`) (`|MakeArray` (struct) :!type "AkExternalSourceInfo Structure") "")
      (`KismetSystemLibrary.Delay` 0.45)
      (if (not (`self.IsChainsawCancelled`))
        (bind _audio_component_2 (message `/Game/Characters/Slashers/Blueprints/Interfaces/ISlasherEffectInterface.GetSlasherAudioComponent` (`self.OwningKiller`)))
        (`AkGameObject.PostAkEvent` _audio_component_2 null 0 (delegate `CustomEvent4`) (`|MakeArray` (struct) :!type "AkExternalSourceInfo Structure") "")))))

(event `rev_start`
  (`AudioComponent.Play` (`self.sfx_chainsaw_attack_start`) 0.0))

(event `CustomEvent3`
  (params (CallbackType :type "EAkCallbackType Enum" :default "EndOfEvent") (CallbackInfo :type "AkCallbackInfo Object Reference")))

(event `CustomEvent4`
  (params (CallbackType :type "EAkCallbackType Enum" :default "EndOfEvent") (CallbackInfo :type "AkCallbackInfo Object Reference")))

(event `AudioEvent_Chainsaw_Rev`
  (if (`KismetMathLibrary.RandomBoolWithWeight` 0.8)
    (if (< (`self.RevMultiContinuouslyPlayedNum`) 3)
      (set `self.RevSingleContinuouslyPlayedNum` 0)
      (`/Engine/EditorBlueprintResources/StandardMacros.IncrementInt` (`self.RevMultiContinuouslyPlayedNum`)
        (:`  `
          (set `self.IsRevMultiPlaying` true)
          (set `self.IsRevSinglePlaying` false)
          (`AudioComponent.FadeIn` (`self.sfx_chainsaw_attack_rev_multi`) (`KismetMathLibrary.SelectFloat` 0.0 0.5 (`self.FirstRevPlayed`)) 1.0 0.0 "Linear")
          (set `self.FirstRevPlayed` true)))
      (else
        (`self.AudioEvent_Chainsaw_Rev`)))
    (elif (< (`self.RevSingleContinuouslyPlayedNum`) 3)
      (set `self.RevMultiContinuouslyPlayedNum` 0)
      (`/Engine/EditorBlueprintResources/StandardMacros.IncrementInt` (`self.RevSingleContinuouslyPlayedNum`)
        (:`  `
          (set `self.IsRevMultiPlaying` false)
          (set `self.IsRevSinglePlaying` true)
          (`AudioComponent.FadeIn` (`self.sfx_chainsaw_attack_rev_single`) (`KismetMathLibrary.SelectFloat` 0.0 0.5 (`self.FirstRevPlayed`)) 1.0 0.0 "Linear")
          (set `self.FirstRevPlayed` true)))
      (else
        (`self.AudioEvent_Chainsaw_Rev`)))))

(event `AudioEvent_Chainsaw_Hit_Object`
  (`self.AudioEvent_Chainsaw_Cancel`)
  (if (`self.IsLocalPlayer`)
    (`GameplayStatics.PlaySoundAtLocation` "/Game/HillbillySounds/SoundWaves/sfx_chainsaw_attack_hit_wall_04.sfx_chainsaw_attack_hit_wall_04" (`self.K2_GetActorLocation` (`self.OwningKiller`)) (struct) 1.0 1.0 0.0 null null null)
    (else
      (bind _audio_component (message `/Game/Characters/Slashers/Blueprints/Interfaces/ISlasherEffectInterface.GetSlasherAudioComponent` (`self.OwningKiller`)))
      (`AkGameObject.PostAkEvent` _audio_component null 0 (delegate `CustomEvent7`) (`|MakeArray` (struct) :!type "AkExternalSourceInfo Structure") ""))))

(event `CustomEvent7`
  (params (CallbackType :type "EAkCallbackType Enum" :default "EndOfEvent") (CallbackInfo :type "AkCallbackInfo Object Reference")))

(event `AudioEvent_Chainsaw_Hit_Survivor`
  (if (`self.IsLocalPlayer`)
    (`AudioComponent.FadeIn` (`self.sfx_chainsaw_attack_body_loop`) 0.0 1.0 0.0 "Linear")
    (`KismetSystemLibrary.Delay` 0.5)
    (`AudioComponent.FadeOut` (`self.sfx_chainsaw_attack_body_loop`) 0.5 0.0 "Linear")
    (else
      (bind _audio_component (message `/Game/Characters/Slashers/Blueprints/Interfaces/ISlasherEffectInterface.GetSlasherAudioComponent` (`self.OwningKiller`)))
      (`AkGameObject.PostAkEvent` _audio_component null 0 (delegate `CustomEvent6`) (`|MakeArray` (struct) :!type "AkExternalSourceInfo Structure") ""))))

(event `CustomEvent6`
  (params (CallbackType :type "EAkCallbackType Enum" :default "EndOfEvent") (CallbackInfo :type "AkCallbackInfo Object Reference")))

(event `AudioEvent_Chainsaw_Stop`
  ;[1 1 1] Duplicate of AudioEvent_Chainsaw_Cancel, but without "chainsaw_stop" sound cue
  (set `self.IsChainsawCancelled` true)
  (if (`self.IsLocalPlayer`)
    (clear `AudioComponent.OnAudioFinished` (`self.sfx_chainsaw_attack_rev_single`))
    (clear `AudioComponent.OnAudioFinished` (`self.sfx_chainsaw_attack_rev_multi`))
    (`KismetSystemLibrary.K2_ClearAndInvalidateTimerHandle` (`self.rev_start_timer`))
    (`KismetSystemLibrary.K2_ClearAndInvalidateTimerHandle` (`self.first_rev_timer`))
    (`AudioComponent.FadeOut` (`self.sfx_chainsaw_attack_rev_single`) 0.5 0.0 "Linear")
    (`AudioComponent.FadeOut` (`self.sfx_chainsaw_attack_rev_multi`) 0.5 0.0 "Linear")
    (`AudioComponent.FadeOut` (`self.sfx_chainsaw_idle_loop`) 0.5 0.0 "Linear")
    (`AudioComponent.FadeOut` (`self.sfx_chainsaw_attack_start_add`) 0.5 0.0 "Linear")
    (`AudioComponent.FadeOut` (`self.sfx_chainsaw_attack_start`) 0.5 0.0 "Linear")
    (set `self.IsRevSinglePlaying` false)
    (set `self.IsRevMultiPlaying` false)
    (set `self.RevSingleContinuouslyPlayedNum` 0)
    (set `self.RevMultiContinuouslyPlayedNum` 0)
    (set `self.FirstRevPlayed` false)
    (else
      (bind _audio_component (message `/Game/Characters/Slashers/Blueprints/Interfaces/ISlasherEffectInterface.GetSlasherAudioComponent` (`self.OwningKiller`)))
      (`AkGameObject.PostAkEvent` _audio_component null 0 (delegate `CustomEvent5`) (`|MakeArray` (struct) :!type "AkExternalSourceInfo Structure") ""))))

(event `CustomEvent5`
  (params (CallbackType :type "EAkCallbackType Enum" :default "EndOfEvent") (CallbackInfo :type "AkCallbackInfo Object Reference")))

(event `self.ReceiveTick`
  (params (DeltaSeconds :type "Float (single-precision)"))
  (bind _asdbdgame_state (cast `DBDGameState` (`GameplayStatics.GetGameState`)))
  (if (`DBDGameState.GetIsGameEnded` _asdbdgame_state)
    (`self.AudioEvent_Chainsaw_Stop`)))

(fn `UserConstructionScript`)