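; BP_Blood is a Blueprint that logs a fullscreen blood activation message on BeginPlay but contains no blood effect logic.
; Tick polls the F key and, while a widget-visible flag is set, passes mouse deltas to CalculateSelectedItem, resembling a radial selection menu.
; CalculateSelectedItem is an empty stub, and the F press and release branches perform no actions.
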(event `self.ReceiveBeginPlay`
  (`/Game/LoggingUtilities/BlueprintLoggingLibrary.PrintString` "FullscreenBlood Activated" "NewEnumerator0" "LogBlueprintUserMessages" true self))

(event `self.ReceiveTick`
  (params (DeltaSeconds :type "Float (single-precision)"))
  (bind (_deltax _deltay) (`PlayerController.GetInputMouseDelta` (`GameplayStatics.GetPlayerController` 0)))
  (if (`PlayerController.WasInputKeyJustPressed` (`GameplayStatics.GetPlayerController` 0) "F")
    _
    (elif (`self.bIsWidgetCurrentlyVisible`)
      (if (not (`PlayerController.WasInputKeyJustReleased` (`GameplayStatics.GetPlayerController` 0) "F"))
        (`self.CalculateSelectedItem` _deltax _deltay)))))

(fn `CalculateSelectedItem`
  (params (MouseDeltaX :type "Float (double-precision)") (MouseDeltaY :type "Float (double-precision)")))

(fn `UserConstructionScript`)