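; BP_CustomizedMesh is a Blueprint that appears to be a debug test for changing material textures on the owning killer's customized head mesh.
; Each tick it checks whether player 0 just pressed C, then loops over the KillerHead skeletal mesh materials.
; For dynamic material instances, it prints the current Main_BaseColor texture name, swaps in the Transparent texture and prints a confirmation.
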(event `self.ReceiveTick`
  (params (DeltaSeconds :type "Float (single-precision)"))
  (if (`PlayerController.WasInputKeyJustPressed` (`GameplayStatics.GetPlayerController` 0) "C")
    (for _array_element (`MeshComponent.GetMaterials` (`CustomizedSkeletalMesh.GetSkeletalMesh` (`DBDBasePlayer.GetCustomizedSkeletalMesh` (`self.OwningKiller`)) "KillerHead"))
      (bind _asmaterial_instance_dynamic (cast `MaterialInstanceDynamic` _array_element))
      (bind _returnvalue (`MaterialInstanceDynamic.K2_GetTextureParameterValue` _asmaterial_instance_dynamic "Main_BaseColor"))
      (`/Game/LoggingUtilities/BlueprintLoggingLibrary.PrintString` (`KismetSystemLibrary.GetDisplayName` _returnvalue) "NewEnumerator0" "LogBlueprintUserMessages" true self)
      (`MaterialInstanceDynamic.SetTextureParameterValue` _asmaterial_instance_dynamic "Main_BaseColor" "/Game/Characters/Slashers/Crooked/Materials/Hair/Transparent.Transparent")
      (`/Game/LoggingUtilities/BlueprintLoggingLibrary.PrintString` "Mat changed" "NewEnumerator0" "LogBlueprintUserMessages" true self))))

(fn `UserConstructionScript`)