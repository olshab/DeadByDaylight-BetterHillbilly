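; A debug-style mod actor that plays killer chainsaw audio on the local player character from numpad keys.
; It enables input on BeginPlay, and NumPad 7, 8 and 9 trigger the startup, rev loop and stop Wwise events.
; Each key fetches the character's slasher audio component through an interface message, posts its event if valid, and prints a label on screen.
; The Wwise callback events are empty stubs.
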(event `self.ReceiveBeginPlay`
  (`self.EnableInput` (`GameplayStatics.GetPlayerController` 0)))

(event `Key|NumPadSeven`
  (params (Key :type "Key Structure"))
  (:`Pressed`
    (bind _audio_component (message `/Game/Characters/Slashers/Blueprints/Interfaces/ISlasherEffectInterface.GetSlasherAudioComponent` (`GameplayStatics.GetPlayerCharacter` 0)))
    (`/Engine/EditorBlueprintResources/StandardMacros.IsValid` _audio_component
      (:`Is Valid`
        (`AkGameObject.PostAkEvent` _audio_component "/Game/Audio/AudioEvents/Powers/AudioEvent_K03_PWR_Chainsaw_Startup.AudioEvent_K03_PWR_Chainsaw_Startup" 0 (delegate `CustomEvent2`) (`|MakeArray` (struct) :!type "AkExternalSourceInfo Structure") "")
        (`/Game/BetterHilbilly_LoggingUtilities/BlueprintLoggingLibrary.PrintString` "Startup")))))

(event `CustomEvent2`
  (params (CallbackType :type "EAkCallbackType Enum" :default "EndOfEvent") (CallbackInfo :type "AkCallbackInfo Object Reference")))

(event `Key|NumPadEight`
  (params (Key :type "Key Structure"))
  (:`Pressed`
    (bind _audio_component (message `/Game/Characters/Slashers/Blueprints/Interfaces/ISlasherEffectInterface.GetSlasherAudioComponent` (`GameplayStatics.GetPlayerCharacter` 0)))
    (`/Engine/EditorBlueprintResources/StandardMacros.IsValid` _audio_component
      (:`Is Valid`
        (`AkGameObject.PostAkEvent` _audio_component "/Game/Audio/AudioEvents/Powers/AudioEvent_K03_PWR_Chainsaw_Rev_Loop_Start.AudioEvent_K03_PWR_Chainsaw_Rev_Loop_Start" 0 (delegate `CustomEvent`) (`|MakeArray` (struct) :!type "AkExternalSourceInfo Structure") "")
        (`/Game/BetterHilbilly_LoggingUtilities/BlueprintLoggingLibrary.PrintString` "Rev_Loop_Start")))))

(event `CustomEvent`
  (params (CallbackType :type "EAkCallbackType Enum" :default "EndOfEvent") (CallbackInfo :type "AkCallbackInfo Object Reference")))

(event `Key|NumPadNine`
  (params (Key :type "Key Structure"))
  (:`Pressed`
    (bind _audio_component (message `/Game/Characters/Slashers/Blueprints/Interfaces/ISlasherEffectInterface.GetSlasherAudioComponent` (`GameplayStatics.GetPlayerCharacter` 0)))
    (`/Engine/EditorBlueprintResources/StandardMacros.IsValid` _audio_component
      (:`Is Valid`
        (`AkGameObject.PostAkEvent` _audio_component "/Game/Audio/AudioEvents/Powers/AudioEvent_K03_PWR_Chainsaw_Stop.AudioEvent_K03_PWR_Chainsaw_Stop" 0 (delegate `CustomEvent_1`) (`|MakeArray` (struct) :!type "AkExternalSourceInfo Structure") "")
        (`/Game/BetterHilbilly_LoggingUtilities/BlueprintLoggingLibrary.PrintString` "Stop")))))

(event `CustomEvent_1`
  (params (CallbackType :type "EAkCallbackType Enum" :default "EndOfEvent") (CallbackInfo :type "AkCallbackInfo Object Reference")))

(fn `UserConstructionScript`)